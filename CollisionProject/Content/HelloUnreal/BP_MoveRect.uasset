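; BP_MoveRect moves its static mesh around a rectangular path in the X-Z plane while triggered by Bp_Mybox overlaps.
; On BeginPlay it binds to overlap dispatchers on every Bp_Mybox, with handlers that call Play and Stop.
; Play runs Updatemove on a looping timer, cleared by Stop or after a delay.
; Updatemove steps the relative location, switching the MoveType direction at each bound.
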(event EventPlay
  (Utilities|Time|SetTimerbyFunctionName 0 "Updatemove" 0.01 true)
  (Utilities|FlowControl|Delay 5e+01)
  (Utilities|Time|ClearTimerbyFunctionName 0 "Updatemove"))

(event EventStop
  (Utilities|Time|ClearTimerbyFunctionName 0 "Updatemove"))

(event EventBeginPlay
  (bind _outactors (Actor|GetAllActorsOfClass "/Game/Collision/BluePrint/Bp_Mybox.Bp_Mybox_C"))
  (for _array_element _outactors
    (EventDispatchers|BindEventtoEventDispatcherBeginOverlap _array_element (EventDispatchers|CreateEvent :!event EventBeginOverlap))
    (EventDispatchers|BindEventtoEventDispatcherEndOverlap _array_element (EventDispatchers|CreateEvent :!event EventEndOverlap))))

(event EventTick
  (params (DeltaSeconds :type Float%20%28single-precision%29)))

(fn ConstructionScript)

(fn Updatemove
  (bind _staticmesh (Variables|Default|GetStaticMesh))
  (switch Utilities|FlowControl|Switch|SwitchonEn_MoveType (Variables|Default|GetMoveType)
    (:NewEnumerator0
      (Transformation|AddRelativeLocation _staticmesh "10.000000, 0, 0" false false)
      (if (> (.x (Variables|/Script/Engine.SceneComponent|GetRelativeLocation (Variables|Default|GetStaticMesh))) 1e+03)
        (Variables|Default|SetMoveType "NewEnumerator1")))
    (:NewEnumerator1
      (Transformation|AddRelativeLocation _staticmesh "0.000000,0.000000,10.000000" false false)
      (if (> (.z (Variables|/Script/Engine.SceneComponent|GetRelativeLocation (Variables|Default|GetStaticMesh))) 1e+03)
        (Variables|Default|SetMoveType "NewEnumerator2")))
    (:NewEnumerator2
      (Transformation|AddRelativeLocation _staticmesh "-10.000000, 0, 0" false false)
      (if (< (.x (Variables|/Script/Engine.SceneComponent|GetRelativeLocation (Variables|Default|GetStaticMesh))) 0.0)
        (Variables|Default|SetMoveType "NewEnumerator3")))
    (:NewEnumerator3
      (Transformation|AddRelativeLocation _staticmesh "-0.000000,0.000000,-10.000000" false false)
      (if (< (.z (Variables|/Script/Engine.SceneComponent|GetRelativeLocation (Variables|Default|GetStaticMesh))) 0.0)
        (Variables|Default|SetMoveType "NewEnumerator0")))))

(fn EventBeginOverlap
  (params (NewParam :type Boolean))
  (CallFunction|Play))

(fn EventEndOverlap
  (params (result :type Boolean))
  (CallFunction|Stop))