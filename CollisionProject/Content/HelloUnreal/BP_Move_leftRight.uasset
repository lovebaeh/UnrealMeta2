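; BP_Move_leftRight is an actor that slides its static mesh back and forth along X while triggered by Bp_Mybox overlaps.
; On BeginPlay it binds to the begin and end overlap dispatchers of every Bp_Mybox, which call Play and Stop.
; A timeline drives the mesh's relative location, flipping IsMoveRight on finish to alternate Play and Reverse in a ping-pong loop until stopped.
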(event EventPlay
  (if (Variables|Default|GetIsMoveRight) :!label _label
    (bind _value (Timeline|타임라인_0 Play)
      (:Update
        (Transformation|SetRelativeLocation (Variables|Default|GetStaticMesh) (Math|Vector|MakeVector (* 1000 _value) 0.0 0.0) false false))
      (:Finished
        (Variables|Default|SetIsMoveRight (not (Variables|Default|GetIsMoveRight)))
        (goto _label)))
    (else
      (Timeline|타임라인_0 Reverse))))

(event EventStop
  (bind _value (Timeline|타임라인_0 Stop)
    (:Update
      (Transformation|SetRelativeLocation (Variables|Default|GetStaticMesh) (Math|Vector|MakeVector (* 1000 _value) 0.0 0.0) false false))
    (:Finished
      (Variables|Default|SetIsMoveRight (not (Variables|Default|GetIsMoveRight)))
      (if (Variables|Default|GetIsMoveRight)
        (Timeline|타임라인_0 Play)
        (else
          (Timeline|타임라인_0 Reverse))))))

(event EventBeginPlay
  (bind _outactors (Actor|GetAllActorsOfClass "/Game/Collision/BluePrint/Bp_Mybox.Bp_Mybox_C"))
  (for _array_element _outactors
    (EventDispatchers|BindEventtoEventDispatcherBeginOverlap _array_element (EventDispatchers|CreateEvent :!event EventBeginOverlap))
    (EventDispatchers|BindEventtoEventDispatcherEndOverlap _array_element (EventDispatchers|CreateEvent :!event EventEndOverlap))))

(event Input|KeyboardEvents|B
  (params (Key :type Key%20Structure :default "None")))

(fn ConstructionScript)

(fn EventBeginOverlap
  (params (bresult :type Boolean))
  (CallFunction|Play))

(fn EventEndOverlap
  (params (result :type Boolean))
  (CallFunction|Stop))