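; Collision test box Blueprint whose Cube2 component logs contact events and starts motion elsewhere when overlapped.
; On begin overlap it loops over MoveRect, calling Play on each element and on MoveLeftRight and RotationBall within the same loop body.
; End overlap and hit only print the components and actor involved, both reusing the "Overlapped" label.
; Disconnected loop and print nodes in the event graph never run.
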(event OnComponentBeginOverlap(Cube2)
  (params (OverlappedComponent :type Primitive%20Component%20Object%20Reference) (OtherActor :type Actor%20Object%20Reference) (OtherComp :type Primitive%20Component%20Object%20Reference) (OtherBodyIndex :type Integer) (bFromSweep :type Boolean) (SweepResult :type Hit%20Result%20Structure%20%28by%20ref%29))
  (Development|PrintString (Utilities|String|Append "Overlapped" (Utilities|GetDisplayName OverlappedComponent) "OtherActor" (Utilities|GetDisplayName OtherActor) "OtherComp" (Utilities|GetDisplayName OtherComp)))
  (for _array_element (Variables|Default|GetMoveRect)
    (Default|Play _array_element)
    (Default|Play (Variables|Default|GetMoveLeftRight))
    (Default|Play (Variables|Default|GetRotationBall))))

(event OnComponentEndOverlap(Cube2)
  (params (OverlappedComponent :type Primitive%20Component%20Object%20Reference) (OtherActor :type Actor%20Object%20Reference) (OtherComp :type Primitive%20Component%20Object%20Reference) (OtherBodyIndex :type Integer))
  (Development|PrintString (Utilities|String|Append "Overlapped" (Utilities|GetDisplayName OverlappedComponent) "OtherActor" (Utilities|GetDisplayName OtherActor) "OtherComp" (Utilities|GetDisplayName OtherComp))))

(event OnComponentHit(Cube2)
  (params (HitComponent :type Primitive%20Component%20Object%20Reference) (OtherActor :type Actor%20Object%20Reference) (OtherComp :type Primitive%20Component%20Object%20Reference) (NormalImpulse :type Vector :default "0, 0, 0") (Hit :type Hit%20Result%20Structure%20%28by%20ref%29))
  (Development|PrintString (Utilities|String|Append "Overlapped" (Utilities|GetDisplayName HitComponent) "OtherActor" (Utilities|GetDisplayName OtherActor) "OtherComp" (Utilities|GetDisplayName OtherComp))))

(event EventBeginPlay)

(fn ConstructionScript)