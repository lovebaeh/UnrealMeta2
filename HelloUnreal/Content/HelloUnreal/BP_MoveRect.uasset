(event EventBeginPlay
  (Utilities|Time|SetTimerbyFunctionName 0 "Updatemove" 0.01 true)
  (Utilities|FlowControl|Delay 5.0)
  (Utilities|Time|ClearTimerbyFunctionName 0 "Updatemove"))

(event EventTick
  (params (DeltaSeconds :type Float%20%28single-precision%29))
  (CallFunction|Updatemove))

(event Input|KeyboardEvents|R
  (params (Key :type Key%20Structure :default "None"))
  (:Pressed
    (Development|PrintString "Hello"))
  (:Released
    (Development|PrintString "Hello")))

(fn ConstructionScript)

(fn Updatemove
  (bind _staticmesh (Variables|Default|GetStaticMesh))
  (switch Utilities|FlowControl|Switch|SwitchonEn_MoveType (Variables|Default|GetMoveType)
    (:NewEnumerator0
      (Transformation|AddRelativeLocation _staticmesh "10.000000, 0, 0" false false)
      (if (> (.x (Variables|/Script/Engine.SceneComponent|GetRelativeLocation (Variables|Default|GetStaticMesh))) 1e+03)
        (Variables|Default|SetMoveType "NewEnumerator1")))
    (:NewEnumerator1
      (Transformation|AddRelativeLocation _staticmesh "0.000000,0.000000,10.000000" false false)
      (if (> (.z (Variables|/Script/Engine.SceneComponent|GetRelativeLocation (Variables|Default|GetStaticMesh))) 1e+03)
        (Variables|Default|SetMoveType "NewEnumerator2")))
    (:NewEnumerator2
      (Transformation|AddRelativeLocation _staticmesh "-10.000000, 0, 0" false false))
    (:NewEnumerator3
      (Transformation|AddRelativeLocation _staticmesh "-0.000000,0.000000,-10.000000" false false)
      (if (< (.z (Variables|/Script/Engine.SceneComponent|GetRelativeLocation (Variables|Default|GetStaticMesh))) 0.0)
        (Variables|Default|SetMoveType "NewEnumerator0")))))